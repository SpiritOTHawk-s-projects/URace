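; BP_VolumetricSplineActor builds a tube from spline meshes along its Spline component, in the VolumetricGlass content.
; The construction script adds one spline mesh per segment, fitting the configurable static mesh and forward axis to each pair of points' local positions and tangents.
; Segments cast no shadow, use a configurable translucency sort priority, and have world-static query and physics collision that blocks the Camera channel.
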(fn `UserConstructionScript`
  (locals (TempMesh :type "SplineMeshComponent Object Reference"))
  (bind _spline (`self.Spline`))
  (bind _spline_2 (`self.Spline`))
  (bind _tempmesh (`local.TempMesh`))
  ;[1 1 1] Create simple tube spline mesh
  (for _index (range (+ (- (`SplineComponent.GetNumberOfSplinePoints` (`self.Spline`)) 2) 1))
    (bind _returnvalue (`AddComponent|NODE_AddSplineMeshComponent-0`))
    (set `local.TempMesh` _returnvalue)
    (`StaticMeshComponent.SetStaticMesh` (`local.TempMesh`) (`self.StaticMesh`))
    (`SplineMeshComponent.SetForwardAxis` _returnvalue (`self.ForwardAxis`) true)
    (`SceneComponent.K2_AttachToComponent` (`local.TempMesh`) (`self.Spline`) "None" "KeepRelative" "KeepRelative" "KeepRelative" true)
    (`PrimitiveComponent.SetCastShadow` (`local.TempMesh`) false)
    (bind _returnvalue_2 (+ _index 1))
    (`SplineMeshComponent.SetStartAndEnd` (`local.TempMesh`) (`SplineComponent.GetLocationAtSplinePoint` _spline_2 _index "Local") (`SplineComponent.GetTangentAtSplinePoint` _spline_2 _index "Local") (`SplineComponent.GetLocationAtSplinePoint` _spline _returnvalue_2 "Local") (`SplineComponent.GetTangentAtSplinePoint` _spline _returnvalue_2 "Local") true)
    (`PrimitiveComponent.SetCollisionEnabled` _tempmesh "QueryAndPhysics")
    (`PrimitiveComponent.SetCollisionObjectType` _tempmesh "ECC_WorldStatic")
    (`PrimitiveComponent.SetTranslucentSortPriority` (`local.TempMesh`) (`self.TranslucencySortPriority`))
    (`PrimitiveComponent.SetCollisionResponseToChannel` (`local.TempMesh`) "ECC_Camera" "ECR_Block")))