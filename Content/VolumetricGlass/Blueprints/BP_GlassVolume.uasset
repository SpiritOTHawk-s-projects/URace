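; BP_GlassVolume defines an axis-aligned box volume for the volumetric glass effect.
; InitMaterial runs at construction and BeginPlay, sizing the box from VolumeExtend and placing a scaled plane on its top face.
; It writes the box's world-space min and max corners to the PC_VolumetricGlass parameter collection, so those bounds are shared globally rather than per instance.
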(event `self.ReceiveBeginPlay`
  (`self.InitMaterial`))

(fn `InitMaterial`
  (bind _volumeextend (`self.VolumeExtend`))
  (bind _box (`self.Box`))
  (bind _returnvalue (`SceneComponent.K2_GetComponentLocation` _box))
  (bind _returnvalue_2 (+ _returnvalue _volumeextend))
  (`BoxComponent.SetBoxExtent` _box _volumeextend true)
  (`KismetMaterialLibrary.SetVectorParameterValue` "/Game/VolumetricGlass/Materials/Utils/PC_VolumetricGlass.PC_VolumetricGlass" "MinVolume" (`KismetMathLibrary.Conv_VectorToLinearColor` (- _returnvalue _volumeextend)))
  (`KismetMaterialLibrary.SetVectorParameterValue` "/Game/VolumetricGlass/Materials/Utils/PC_VolumetricGlass.PC_VolumetricGlass" "MaxVolume" (`KismetMathLibrary.Conv_VectorToLinearColor` _returnvalue_2))
  (`SceneComponent.K2_SetWorldLocation` (`self.Plane`) (`KismetMathLibrary.MakeVector` (.x _returnvalue) (.y _returnvalue) (.z _returnvalue_2)) false false)
  (`SceneComponent.SetWorldScale3D` (`self.Plane`) (* (`self.VolumeExtend`) 0.02)))

(fn `UserConstructionScript`
  (`self.InitMaterial`))